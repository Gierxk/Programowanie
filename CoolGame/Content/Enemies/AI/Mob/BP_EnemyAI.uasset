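; Mob enemy Blueprint that reports player proximity to its AI blackboard and deals melee damage.
; Each tick it updates the in-range key and, while the blackboard's attacking key is set, sphere-traces at the left-hand socket.
; A hit list limits damage to once per BP_BaseCharacter until Attack clears it and plays the light attack montage.
; TryTakeDamage damages BPCStats directly but is not called here; GetHit is empty.
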(event EventBeginPlay
  (AI|Components|Blackboard|SetValueasBool (AI|GetBlackboard 0) (Utilities|Name|MakeLiteralName "isAttacking?") false))

(event EventTick
  (params (DeltaSeconds :type Float%20%28single-precision%29))
  (bind _handl (Variables|Default|GetHandL))
  (bind _hit_actor (Variables|Default|GetHit%20Actor))
  (bind _returnvalue (Transformation|GetSocketLocation _handl "hand_l"))
  (CallFunction|CheckIsinRange)
  (if (ScalableFloat|GetValueasBool (AI|GetBlackboard 0) (Utilities|Name|MakeLiteralName "isAttacking?"))
    (bind (_outhits _returnvalue_2) (Collision|MultiSphereTraceForObjects _returnvalue _returnvalue 2e+01 (Utilities|Array|MakeArray "ObjectTypeQuery8") false (Utilities|Array|MakeArray self 0) "ForDuration" true "(R=1.000000,G=0.000000,B=0.000000,A=1.000000)" "(R=0.000000,G=1.000000,B=0.000000,A=1.000000)" 3.0))
    (if _returnvalue_2
      (for _array_element _outhits
        (Utilities|IsValid (.HitActor (Collision|BreakHitResult _array_element))
          (:Is%20Valid
            (if (and (not (Utilities|Array|ContainsItem _hit_actor (.HitActor (Collision|BreakHitResult _array_element)))) (Class|GameplayStatics|ObjectIsA (.HitActor (Collision|BreakHitResult _array_element)) "/Game/Blueprints/Characters/BP_BaseCharacter.BP_BaseCharacter_C"))
              (Utilities|Array|AddUnique _hit_actor (.HitActor (Collision|BreakHitResult _array_element)))
              (Game|Damage|ApplyDamage (.HitActor (Collision|BreakHitResult _array_element)) 1e+01 0 0))))))))

(fn ConstructionScript)

(fn TryTakeDamage
  (params (hitObject :type Object%20Object%20Reference))
  (Utilities|FlowControl|Sequence
    (:then_0
      (bind _asbp_base_character (Utilities|Casting|CastToBP_BaseCharacter hitObject))
      (Default|TakeDamage (Variables|/Game/Blueprints/Characters/BP_BaseCharacter.BP_BaseCharacter_C|GetBPC_Stats _asbp_base_character) 1e+01))))

(fn CheckIsinRange
  (bind _returnvalue (Utilities|Name|MakeLiteralName "isInRange?"))
  (bind _self self)
  (bind _returnvalue_2 (AI|GetAIController _self))
  (bind _returnvalue_3 (AI|GetBlackboard _returnvalue_2))
  (if (<= (Transformation|GetDistanceTo (Game|GetPlayerCharacter 0)) (Variables|Default|Getrange))
    (AI|Components|Blackboard|SetValueasBool _returnvalue_3 _returnvalue true)
    (return true)
    (else
      (AI|Components|Blackboard|SetValueasBool _returnvalue_3 _returnvalue false)
      (return false))))

(fn Attack
  (bind _returnvalue (Animation|PlayAnimMontage "/Game/Animations/LightAttacks/AM_LightAttack_1.AM_LightAttack_1" 1.0 "None"))
  (Variables|Default|SetisAttacking? true)
  (Utilities|Array|Clear (Variables|Default|GetHit%20Actor))
  (return _returnvalue))

(fn GetHit
  (return 0))