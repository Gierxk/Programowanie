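; AI controller for the boss enemy that starts the BT_EnemyBoss behavior tree on BeginPlay and feeds its blackboard.
; Every Tick it sets the "canAttack?" key by whether the player character is within Range.
; When PawnSensing sees a pawn, it sets "seeingTarget?" true and stores that pawn as "targetActor", with no logic here to clear either key.
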(event OnSeePawn(PawnSensing)
  (params (Pawn :type Pawn%20Object%20Reference))
  (bind _returnvalue (AI|GetBlackboard 0))
  (AI|Components|Blackboard|SetValueasBool _returnvalue (Utilities|Name|MakeLiteralName "seeingTarget?") true)
  (AI|Components|Blackboard|SetValueasObject _returnvalue (Utilities|Name|MakeLiteralName "targetActor") Pawn))

(event EventBeginPlay
  (AI|RunBehaviorTree "/Game/Enemies/AI/Boss/BT_EnemyBoss.BT_EnemyBoss"))

(event EventTick
  (params (DeltaSeconds :type Float%20%28single-precision%29))
  (bind _returnvalue (Utilities|Name|MakeLiteralName "canAttack?"))
  (bind _returnvalue_2 (AI|GetBlackboard 0))
  (if (<= (Transformation|GetDistanceTo (Game|GetPlayerCharacter 0)) (Variables|Default|GetRange))
    (AI|Components|Blackboard|SetValueasBool _returnvalue_2 _returnvalue true)
    (else
      (AI|Components|Blackboard|SetValueasBool _returnvalue_2 _returnvalue false))))

(fn ConstructionScript)