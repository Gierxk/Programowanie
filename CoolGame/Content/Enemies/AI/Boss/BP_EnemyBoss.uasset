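; Boss enemy Blueprint that handles melee attacks and binds the boss health bar to its stats component.
; Attack plays a heavy montage, sets IsAttacking and clears the hit list.
; While the separate blackboard attack flag is true, Tick sphere-traces between hand sockets with debug drawing, damaging each new BP_BaseCharacter once.
; TryTakeDamage instead damages a passed character through its stats component; GetHit is an empty stub.
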(event EventBeginPlay
  (AI|Components|Blackboard|SetValueasBool (AI|GetBlackboard 0) (Utilities|Name|MakeLiteralName "isAttacking?") false)
  (Variables|/Game/Blueprints/Components/BPC_Stats.BPC_Stats_C|SetHealthBar (Variables|Default|GetBPC_Stats) "/Game/HUD/Widgets/WBP_BossHealthBar.WBP_BossHealthBar"))

(event EventTick
  (params (DeltaSeconds :type Float%20%28single-precision%29))
  (bind _hand (Variables|Default|GetHand))
  (bind _hit_actor (Variables|Default|GetHit%20Actor))
  (if (ScalableFloat|GetValueasBool (AI|GetBlackboard 0) (Utilities|Name|MakeLiteralName "isAttacking?"))
    (bind (_outhits _returnvalue) (Collision|MultiSphereTraceForObjects (Transformation|GetSocketLocation _hand "start") (Transformation|GetSocketLocation _hand "end") 2e+01 (Utilities|Array|MakeArray "ObjectTypeQuery8") false (Utilities|Array|MakeArray self 0) "ForDuration" true "(R=1.000000,G=0.000000,B=0.000000,A=1.000000)" "(R=0.000000,G=1.000000,B=0.000000,A=1.000000)" 3.0))
    (if _returnvalue
      (for _array_element _outhits
        (Utilities|IsValid (.HitActor (Collision|BreakHitResult _array_element))
          (:Is%20Valid
            (if (and (not (Utilities|Array|ContainsItem _hit_actor (.HitActor (Collision|BreakHitResult _array_element)))) (Class|GameplayStatics|ObjectIsA (.HitActor (Collision|BreakHitResult _array_element)) "/Game/Blueprints/Characters/BP_BaseCharacter.BP_BaseCharacter_C"))
              (Utilities|Array|AddUnique _hit_actor (.HitActor (Collision|BreakHitResult _array_element)))
              (Game|Damage|ApplyDamage (.HitActor (Collision|BreakHitResult _array_element)) 1e+01 0 0))))))))

(fn ConstructionScript)

(fn TryTakeDamage
  (params (hitObject :type Object%20Object%20Reference))
  (Utilities|FlowControl|Sequence
    (:then_0
      (bind _asbp_base_character (Utilities|Casting|CastToBP_BaseCharacter hitObject))
      (Default|TakeDamage (Variables|/Game/Blueprints/Characters/BP_BaseCharacter.BP_BaseCharacter_C|GetBPC_Stats _asbp_base_character) 1e+01))))

(fn Attack
  (bind _returnvalue (Animation|PlayAnimMontage "/Game/Animations/HeavyAttacks/AM_HeavyAttack_1.AM_HeavyAttack_1" 1.0 "None"))
  (Variables|Default|SetisAttacking? true)
  (Utilities|Array|Clear (Variables|Default|GetHit%20Actor))
  (return _returnvalue))

(fn GetHit
  (return 0))