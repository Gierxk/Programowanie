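; Enemy Blueprint that feeds perception and range state into its AI controller's Blackboard.
; Tick sets "isInRange?" by comparing distance to the player against Range.
; PawnSensing sight of a BP_BaseCharacter sets "seePlayer?", which a retriggerable delay clears one second after the last sighting.
; "alarmed?" turns true unconditionally shortly after BeginPlay, and heard noises only print their location.
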(event OnSeePawn(PawnSensing)
  (params (Pawn :type Pawn%20Object%20Reference))
  (Utilities|Casting|CastToBP_BaseCharacter Pawn)
  (CallFunction|SetDetectPlayerState))

(event OnHearNoise(PawnSensing)
  (params (Instigator :type Pawn%20Object%20Reference) (Location :type Vector%20%28by%20ref%29 :default "0, 0, 0") (Volume :type Float%20%28single-precision%29))
  (Development|PrintString (Utilities|String|ToString(Vector) Location)))

(event Custom|SetDetectPlayerState
  (AI|Components|Blackboard|SetValueasBool (AI|GetBlackboard (Pawn|GetController)) (Utilities|Name|MakeLiteralName "seePlayer?") true)
  (Utilities|FlowControl|RetriggerableDelay 1.0)
  (AI|Components|Blackboard|SetValueasBool (AI|GetBlackboard (Pawn|GetController)) (Utilities|Name|MakeLiteralName "seePlayer?") false))

(event EventBeginPlay
  (Utilities|FlowControl|Delay 5.0)
  (Development|PrintString "Hello")
  (AI|Components|Blackboard|SetValueasBool (AI|GetBlackboard (Pawn|GetController)) (Utilities|Name|MakeLiteralName "alarmed?") true))

(event Collision|EventActorBeginOverlap
  (params (OtherActor :type Actor%20Object%20Reference)))

(event EventTick
  (params (DeltaSeconds :type Float%20%28single-precision%29))
  (bind _returnvalue (Pawn|GetController))
  (bind _returnvalue_2 (Utilities|Name|MakeLiteralName "isInRange?"))
  (bind _returnvalue_3 (AI|GetBlackboard _returnvalue))
  (if (< (Transformation|GetDistanceTo (Game|GetPlayerCharacter 0)) (Variables|Default|Getrange))
    (AI|Components|Blackboard|SetValueasBool _returnvalue_3 _returnvalue_2 true)
    (else
      (AI|Components|Blackboard|SetValueasBool _returnvalue_3 _returnvalue_2 false))))

(fn ConstructionScript)