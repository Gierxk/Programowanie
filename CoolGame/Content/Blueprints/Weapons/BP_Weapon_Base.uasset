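; Base melee weapon Blueprint that handles hit detection and light-attack combo selection.
; While collision is active, Tick sphere-traces between the mesh's Start and End sockets, damaging each BP_BaseEnemy once per swing via a HitActors list.
; PerformLightAttack returns the next montage or animation from AttackAnims, advancing the combo index.
; The combo resets after the final attack or when a retriggerable delay expires.
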(event Custom|Attack
  ;[0.15 0.15 0.15 0.5] Combo Events
  (Math|Integer|IncrementInt (Variables|Default|GetAttack%20Combo%20Index)
    (:%20%20
      (Utilities|FlowControl|RetriggerableDelay 2.0)
      (Variables|Default|SetAttack%20Combo%20Index 0))))

(event Custom|ResetCombo
  ;[0.15 0.15 0.15 0.5] Combo Events
  (Variables|Default|SetAttack%20Combo%20Index 0))

(event Custom|StartWeaponCollision
  ;[0.15 0.15 0.15 0.5] Weapon Trace
  (Utilities|Array|Clear (Variables|Default|GetHit%20Actors))
  (Variables|Default|SetWeapon%20Collision%20Active? true))

(event Custom|EndWeaponCollision
  ;[0.15 0.15 0.15 0.5] Weapon Trace
  (Variables|Default|SetWeapon%20Collision%20Active? false))

(event EventTick
  (params (DeltaSeconds :type Float%20%28single-precision%29))
  (bind _weaponmesh (Variables|Default|GetWeaponMesh))
  (bind _hit_actors (Variables|Default|GetHit%20Actors))
  ;[0.15 0.15 0.15 0.5] Weapon Trace
  (if (Variables|Default|GetWeapon%20Collision%20Active?)
    (bind (_outhits _returnvalue) (Collision|MultiSphereTraceForObjects (Transformation|GetSocketLocation _weaponmesh "Start") (Transformation|GetSocketLocation _weaponmesh "End") 2e+01 (Utilities|Array|MakeArray "ObjectTypeQuery3") false (Utilities|Array|MakeArray self (Game|Player|GetPlayerPawn 0)) "ForDuration"))
    (if _returnvalue
      (for _array_element _outhits
        (Utilities|IsValid (.HitActor (Collision|BreakHitResult _array_element))
          (:Is%20Valid
            (if (and (not (Utilities|Array|ContainsItem _hit_actors (.HitActor (Collision|BreakHitResult _array_element)))) (Class|GameplayStatics|ObjectIsA (.HitActor (Collision|BreakHitResult _array_element)) "/Game/Enemies/BP_BaseEnemy.BP_BaseEnemy_C"))
              (Utilities|Array|AddUnique _hit_actors (.HitActor (Collision|BreakHitResult _array_element)))
              (Game|Damage|ApplyDamage (.HitActor (Collision|BreakHitResult _array_element)) 35.0 (Game|GetPlayerController 0) self))))))))

(fn ConstructionScript)

(fn PerformLightAttack
  (bind _attack_anims (Variables|Default|GetAttack%20Anims))
  (if (>= (Variables|Default|GetAttack%20Combo%20Index) (- (Utilities|Array|Length (Variables|Default|GetAttack%20Anims)) 1))
    (CallFunction|ResetCombo)
    (return (Utilities|Array|Get(acopy) _attack_anims (Utilities|Array|LastIndex _attack_anims)))
    (else
      (CallFunction|Attack)
      (return (Utilities|Array|Get(acopy) (Variables|Default|GetAttack%20Anims) (- (Variables|Default|GetAttack%20Combo%20Index) 1))))))