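; Base actor Blueprint for insight items that can be hidden and revealed in the game.
; It starts hidden on BeginPlay by calling HideItem.
; Paired HideItem and ShowItem events toggle the mesh's visibility and collision and the root component's active state.
; Nothing in this Blueprint calls ShowItem.
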(event Custom|ShowItem
  (bind _mesh (Variables|Default|GetMesh))
  (Rendering|SetVisibility _mesh true false)
  (Collision|SetCollisionEnabled _mesh "QueryAndPhysics")
  (Components|Activation|SetActive (Variables|Default|GetDefaultSceneRoot) true false))

(event Custom|HideItem
  (bind _mesh (Variables|Default|GetMesh))
  (Rendering|SetVisibility _mesh false false)
  (Collision|SetCollisionEnabled _mesh "NoCollision")
  (Components|Activation|SetActive (Variables|Default|GetDefaultSceneRoot) false false))

(event EventBeginPlay
  (CallFunction|HideItem))

(event Collision|EventActorBeginOverlap
  (params (OtherActor :type Actor%20Object%20Reference)))

(event EventTick
  (params (DeltaSeconds :type Float%20%28single-precision%29)))

(fn ConstructionScript)