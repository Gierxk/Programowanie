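; BPC_Stats is a stats component that tracks health, death, poise and stagger state.
; TakeDamage lowers health and flags death at zero, while TakeDamagePoise builds poise damage up to a maximum that triggers stagger.
; A one-second timer, guarded against restarting by CanBeStaggered, then clears poise and stagger.
; A separate Staggered function returns damage scaled by 1.5, though nothing in this file calls it.
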(event EventBeginPlay)

(event EventTick
  (params (DeltaSeconds :type Float%20%28single-precision%29)))

(fn TakeDamage
  (params (Damage :type Float%20%28double-precision%29))
  (bind _output_get (Variables|HP|SetCurrentHealth (- (Variables|HP|GetCurrentHealth) Damage)))
  (if (<= _output_get 0.0)
    (Variables|HP|SetCurrentHealth 0.0)
    (Variables|HP|SetIsDead? true)))

(fn TakeDamagePoise
  (params (PoiseDamage :type Float%20%28double-precision%29))
  (bind _output_get (Variables|Poise|SetCurrentPoise (+ (Variables|Poise|GetCurrentPoise) PoiseDamage)))
  (if (>= _output_get (Variables|Poise|GetMaxPoise))
    (Variables|Poise|SetCurrentPoise (Variables|Poise|GetMaxPoise))
    (Variables|Poise|SetStaggered? true)
    (CallFunction|ResetPoiseStart)))

(fn ResetPoiseStart
  (if (Variables|Poise|GetCanBeStaggered?)
    (Variables|Poise|SetCanBeStaggered? false)
    (bind _returnvalue (Utilities|Time|SetTimerbyFunctionName 0 "ResetPoise" 1.0))
    (Variables|Poise|SetPoiseTimerHandle _returnvalue)))

(fn ResetPoise
  (Variables|Poise|SetCurrentPoise 0.0)
  (Variables|Poise|SetCanBeStaggered? true)
  (Variables|Poise|SetStaggered? false)
  (Utilities|Time|ClearandInvalidateTimerbyHandle (Variables|Poise|GetPoiseTimerHandle)))

(fn Staggered
  (params (InDamage :type Float%20%28double-precision%29))
  (return (* InDamage 1.5)))