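; Base character Blueprint for melee combat with two swappable weapons and buffered light attacks.
; On BeginPlay it spawns a katana and a sword on the same mesh socket, and input toggles which is enabled.
; Attacks play the current weapon's montage; a state enum gates them, saving input for the SaveLightAttack event to replay, while ResetState clears state and combo index.
; A debug key damages the character through its stats component.
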(event Custom|SaveLightAttack
  (if (Variables|Default|GetbSaveLightAttack)
    (Variables|Default|SetbSaveLightAttack false)
    (if (StateMachine|IsStateEqualtoAny (Utilities|Array|MakeArray "NewEnumerator1"))
      (StateMachine|SetState "NewEnumerator0")
      (CallFunction|LightAttackEvent))))

(event Custom|LightAttackEvent
  ;[0.15 0.15 0.15 0.5] Current Weapon Light Attack
  (if (not (StateMachine|IsStateEqualtoAny (Utilities|Array|MakeArray "NewEnumerator1")))
    (bind _attackanim (Default|PerformLightAttack (Variables|Default|GetCurrentWeapon)))
    (Animation|PlayAnimMontage _attackanim 1.0 "None")))

(event Custom|ResetState
  (StateMachine|SetState "NewEnumerator0")
  (Variables|Attack|SetAttackComboIndex 0)
  (Variables|Default|SetbSaveLightAttack false))

(event Input|EnhancedActionEvents|EnhancedInputActionIA_Attack
  (params (ActionValue :type Boolean) (ElapsedSeconds :type Float%20%28double-precision%29) (TriggeredSeconds :type Float%20%28double-precision%29) (InputAction :type Input%20Action%20Object%20Reference :default "/Game/Input/Actions/IA_Attack.IA_Attack"))
  ;[0.15 0.15 0.15 0.5] Attack
  (if (StateMachine|IsStateEqualtoAny (Utilities|Array|MakeArray "NewEnumerator1"))
    (Variables|Default|SetbSaveLightAttack true)
    (else
      (CallFunction|LightAttackEvent))))

(event Input|EnhancedActionEvents|EnhancedInputActionIA_WeaponSwap
  (params (ActionValue :type Boolean) (ElapsedSeconds :type Float%20%28double-precision%29) (TriggeredSeconds :type Float%20%28double-precision%29) (InputAction :type Input%20Action%20Object%20Reference :default "/Game/Input/Actions/IA_WeaponSwap.IA_WeaponSwap"))
  (bind _weapons (Variables|Default|GetWeapons))
  ;[0.15 0.15 0.15 0.5] Weapon Swap
  (Default|DisableWeapon (Variables|Default|GetCurrentWeapon))
  (Utilities|FlowControl|FlipFlop
    (:A
      (Variables|Default|SetCurrentWeapon (Utilities|Array|Get(acopy) _weapons 1)))
    (:B
      (Variables|Default|SetCurrentWeapon (Utilities|Array|Get(acopy) _weapons))))
  (Default|EnableWeapon (Variables|Default|GetCurrentWeapon)))

(event EventBeginPlay
  ;[0.15 0.15 0.15 0.5] Inst Weapons on start
  (CallFunction|SetWeapon))

(event Input|KeyboardEvents|DebugKeyX
  (params (Key :type Key%20Structure :default "None") (ActionValue :type Input%20Action%20Value%20Structure))
  (bind _bpc_stats (Variables|Default|GetBPC_Stats))
  ;[0.15 0.15 0.15 0.5] Dmg test
  (:Pressed
    (Default|TakeDamage _bpc_stats 2e+01)
    (Development|PrintString (Utilities|String|ToString(Float) (Variables|/Game/Blueprints/Components/BPC_Stats.BPC_Stats_C|GetCurrentHealth _bpc_stats)))))

(fn ConstructionScript)

(fn SetState
  (params (NewState :type E_States%20Enum :default "NewEnumerator0"))
  (if (Utilities|Enum|NotEqual(Enum) NewState (Variables|Default|GetCurrentState))
    (Variables|Default|SetCurrentState NewState)))

(fn GetState
  (return (Variables|Default|GetCurrentState)))

(fn IsStateEqualtoAny
  (params (StatesToCheck :type Array%20of%20E_States%20Enums :default "NewEnumerator0"))
  (return (Utilities|Array|ContainsItem StatesToCheck (Variables|Default|GetCurrentState))))

(fn SetWeapon
  (bind _weapons (Variables|Default|GetWeapons))
  (bind _returnvalue (Game|SpawnActorfromClass "/Game/Blueprints/Weapons/BP_Katana.BP_Katana_C" (Math|Transform|MakeTransform "0, 0, 0" "0, 0, 0" "1.000000,1.000000,1.000000") "AlwaysSpawn" "MultiplyWithRoot" 0 0))
  (bind _output_get (Variables|Default|SetCurrentWeapon _returnvalue))
  (Utilities|Array|Add (Variables|Default|GetWeapons) _output_get)
  (Collision|IgnoreActorwhenMoving (Variables|Collision|GetCapsuleComponent) _output_get true)
  (Collision|IgnoreActorwhenMoving (Variables|/Game/Blueprints/Weapons/BP_Weapon_Base.BP_Weapon_Base_C|GetWeaponMesh _output_get) self true)
  (Transformation|AttachComponentToComponent _output_get (Variables|Character|GetMesh) "Weapon_Socket" "KeepRelative" "KeepRelative" "KeepRelative" true)
  (Default|EnableWeapon _output_get)
  (bind _returnvalue_2 (Game|SpawnActorfromClass "/Game/Blueprints/Weapons/BP_Sword.BP_Sword_C" (Math|Transform|MakeTransform "0, 0, 0" "0, 0, 0" "1.000000,1.000000,1.000000") "AlwaysSpawn" "MultiplyWithRoot" 0 0))
  (bind _returnvalue_3 (Utilities|Array|Add _weapons _returnvalue_2))
  (Collision|IgnoreActorwhenMoving (Variables|Collision|GetCapsuleComponent) (Utilities|Array|Get(acopy) _weapons _returnvalue_3) true)
  (Collision|IgnoreActorwhenMoving (Variables|/Game/Blueprints/Weapons/BP_Weapon_Base.BP_Weapon_Base_C|GetWeaponMesh (Utilities|Array|Get(acopy) _weapons _returnvalue_3)) self true)
  (Transformation|AttachComponentToComponent (Utilities|Array|Get(acopy) _weapons _returnvalue_3) (Variables|Character|GetMesh) "Weapon_Socket" "KeepRelative" "KeepRelative" "KeepRelative" true)
  (Default|DisableWeapon (Utilities|Array|Get(acopy) _weapons _returnvalue_3)))